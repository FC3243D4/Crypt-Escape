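; Player combat component for BP_ThirdPersonCharacter that handles target lock, sword attacks and dodging.
; Lock-on sphere-traces from the camera for a living BP_Enemy, attaches a marker, steers control rotation each tick and switches movement to strafing.
; Attacks play one combo montage whose notifies continue only on buffered input and sufficient stamina.
; Dodges pick a directional montage while locked, otherwise forward; both actions spend stamina unless in god mode and pause its regeneration.
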(event `self.ReceiveBeginPlay`
  ;[1 1 1] get player and promote it to variable Player BP
  (bind _asbp_third_person_character (cast `/Game/ThirdPerson/Blueprints/BP_ThirdPersonCharacter` (`self.GetOwner`)))
  (set `self.Player BP` _asbp_third_person_character))

(event `EnhancedInput|/Game/ThirdPerson/Input/Actions/IA_Lock`
  (params (ActionValue :type Boolean) (ElapsedSeconds :type "Float (double-precision)") (TriggeredSeconds :type "Float (double-precision)") (InputAction :type "InputAction Object Reference" :default "/Game/ThirdPerson/Input/Actions/IA_Lock.IA_Lock"))
  (bind _returnvalue (`Actor.GetTransform` (`self.Target Lock Actor`)))
  (bind _transformcomponent (`PlayerCameraManager.TransformComponent` (`GameplayStatics.GetPlayerCameraManager` 0)))
  (bind _charactermovement (`Character.CharacterMovement` (`self.Player BP`)))
  (bind _charactermovement_2 (`Character.CharacterMovement` (`self.Player BP`)))
  (bind (_returnvalue_x _returnvalue_y _returnvalue_z) (`KismetMathLibrary.BreakVector` (`SceneComponent.K2_GetComponentLocation` _transformcomponent)))
  ;[1 1 1] Lock system
  ;;[1 1 1] searcher for actor to lock on in specified area if not already locked
  (:`Started`
    (`self.Target Lock Actor`
      (:`then`
        ;;[1 1 1] if already locked it sets target actor to empty to unlock camera and free the movement direction
        (set `self.Target Lock Actor` null)
        (set `CharacterMovementComponent.bOrientRotationToMovement` true _charactermovement_2)
        (set `CharacterMovementComponent.bUseControllerDesiredRotation` false _charactermovement_2)
        ;;[1 1 1] removes lock icon
        (`Actor.K2_DestroyActor` (`self.TargetLockWidget`)))
      (:`else`
        (bind (_outhit _returnvalue_2) (`KismetSystemLibrary.SphereTraceSingleForObjects` :`Start` (`KismetMathLibrary.MakeVector` _returnvalue_x _returnvalue_y _returnvalue_z) :`End` (+ (`KismetMathLibrary.MakeVector` _returnvalue_x _returnvalue_y (+ _returnvalue_z 35.0)) (* (`KismetMathLibrary.GetForwardVector` (`SceneComponent.K2_GetComponentRotation` _transformcomponent)) 1500.0)) :`Radius` 250.0 :`ObjectTypes` (`|MakeArray` "ObjectTypeQuery3" :!type "EObjectTypeQuery Enum") :`DrawDebugType` "ForDuration" :`DrawTime` 2.0))
        (bind (_bblockinghit _binitialoverlap _time _distance _location _impactpoint _normal _impactnormal _physmat _hitactor) (`GameplayStatics.BreakHitResult` _outhit))
        ;;[1 1 1] if actor found it is promoted to variable target lock actor
        (bind _asbp_enemy (cast `/Game/Blueprints/AI/BP_Enemy` _hitactor))
        (if (and (not (`/Game/Blueprints/AI/BP_Enemy.isDead` _asbp_enemy)) _returnvalue_2)
          (set `self.Target Lock Actor` _hitactor)
          ;;[1 1 1] Set movement around locked actor
          (set `CharacterMovementComponent.bOrientRotationToMovement` false _charactermovement)
          (set `CharacterMovementComponent.bUseControllerDesiredRotation` true _charactermovement)
          ;;[1 1 1] spawns lock icon
          (bind _returnvalue_3 (`|SpawnActorFromClass` "/Game/Blueprints/BP_TargetLockWidget.BP_TargetLockWidget_C" (`KismetMathLibrary.MakeTransform` (`KismetMathLibrary.MakeVector` (.x (.location _returnvalue)) (.y (.location _returnvalue)) (+ (.z (.location _returnvalue)) 50.0)) (.rotation _returnvalue)) "AlwaysSpawn" "MultiplyWithRoot" null null))
          (bind _output_get (set `self.TargetLockWidget` _returnvalue_3))
          (`Actor.K2_AttachToActor` _output_get (`self.Target Lock Actor`) "None" "SnapToTarget" "SnapToTarget" "SnapToTarget" true))))))

(event `self.ReceiveTick`
  (params (DeltaSeconds :type "Float (single-precision)"))
  (bind _charactermovement (`Character.CharacterMovement` (`self.Player BP`)))
  (bind (_returnvalue_roll _returnvalue_pitch _returnvalue_yaw) (`KismetMathLibrary.BreakRotator` (`KismetMathLibrary.FindLookAtRotation` (`Actor.K2_GetActorLocation` (`self.Player BP`)) (`Actor.K2_GetActorLocation` (`self.Target Lock Actor`)))))
  ;[1 1 1] Lock system
  ;;[1 1 1] if lockable pawn found then lock camera onto it
  (bind _target_lock_actor (`self.Target Lock Actor`)
    (:`then`
      (bind _asbp_enemy (cast `/Game/Blueprints/AI/BP_Enemy` _target_lock_actor))
      (if (not (`/Game/Blueprints/AI/BP_Enemy.isDead` _asbp_enemy))
        (`Controller.SetControlRotation` (`Pawn.GetController` (`self.Player BP`)) (`KismetMathLibrary.MakeRotator` _returnvalue_roll (+ _returnvalue_pitch -25.0) _returnvalue_yaw))
        (else
          ;;[1 1 1] if enemy dead unlock camera
          (set `CharacterMovementComponent.bOrientRotationToMovement` true _charactermovement)
          (set `CharacterMovementComponent.bUseControllerDesiredRotation` false _charactermovement)
          (set `self.Target Lock Actor` null)
          (`SceneComponent.SetVisibility` (`/Game/Blueprints/BP_TargetLockWidget.Widget` (`self.TargetLockWidget`)) false false))))
    (:`else`)))

(event `EnhancedInput|/Game/ThirdPerson/Input/Actions/IA_Attack`
  (params (ActionValue :type Boolean) (ElapsedSeconds :type "Float (double-precision)") (TriggeredSeconds :type "Float (double-precision)") (InputAction :type "InputAction Object Reference" :default "/Game/ThirdPerson/Input/Actions/IA_Attack.IA_Attack"))
  (bind _player_bp (`self.Player BP`))
  (bind _player_bp_2 (`self.Player BP`))
  (bind _lighattackstaminacost (`self.LighAttackStaminaCost`))
  (bind _bpc_stats (`/Game/ThirdPerson/Blueprints/BP_ThirdPersonCharacter.BPC_Stats` (`self.Player BP`)))
  (bind _returnvalue (<= _lighattackstaminacost (`/Game/Blueprints/BPC_Stats.Stamina` (`/Game/ThirdPerson/Blueprints/BP_ThirdPersonCharacter.BPC_Stats` _player_bp_2))))
  ;[1 1 1] light attack animation
  (:`Started`
    (`KismetArrayLibrary.Array_Clear` (`/Game/ThirdPerson/Blueprints/BP_ThirdPersonCharacter.hit enemies` _player_bp_2))
    (if (and (not (`self.isAttacking`)) _returnvalue (`/Game/ThirdPerson/Blueprints/BP_ThirdPersonCharacter.weapon equipped` _player_bp_2))
      (set `self.isAttacking` true)
      (`|PlayMontage` (`Character.Mesh` (`self.Player BP`)) "/Game/Characters/Souls/Combat/SwordAttackCombo_Montage.SwordAttackCombo_Montage"
        (:`then`
          (set `/Game/Blueprints/BPC_Stats.regainStamina` false _bpc_stats)
          (if (not (`/Game/ThirdPerson/Blueprints/BP_ThirdPersonCharacter.god mode` _player_bp)) :!label _label
            (`/Game/Blueprints/BPC_Stats.increase value` _bpc_stats "NewEnumerator1" (* _lighattackstaminacost -1.0))))
        (:`OnCompleted`
          (set `/Game/Blueprints/BPC_Stats.regainStamina` true _bpc_stats :!label _label_2)
          (set `self.isAttacking` false)
          (`KismetSystemLibrary.Delay` 1.0)
          (set `self.Combo` false))
        (:`OnInterrupted`
          (goto _label_2))
        (:`OnNotifyBegin`
          (if (and true (`self.Combo`) _returnvalue)
            (set `self.Combo` false)
            (goto _label)
            (else
              (`AnimInstance.Montage_Stop` (`SkeletalMeshComponent.GetAnimInstance` (`Character.Mesh` _player_bp)) 0.2 "/Game/Characters/Souls/Combat/SwordAttackCombo_Montage.SwordAttackCombo_Montage")))))
      (else
        (set `self.Combo` true)))))

(event `EnhancedInput|/Game/ThirdPerson/Input/Actions/IA_Dodge`
  (params (ActionValue :type Boolean) (ElapsedSeconds :type "Float (double-precision)") (TriggeredSeconds :type "Float (double-precision)") (InputAction :type "InputAction Object Reference" :default "/Game/ThirdPerson/Input/Actions/IA_Dodge.IA_Dodge"))
  (bind _dodgestaminacost (`self.DodgeStaminaCost`))
  (bind _player_bp (`self.Player BP`))
  (bind _bpc_stats (`/Game/ThirdPerson/Blueprints/BP_ThirdPersonCharacter.BPC_Stats` _player_bp))
  ;[1 1 1] Dodge
  (:`Triggered`
    (if (and (<= _dodgestaminacost (`/Game/Blueprints/BPC_Stats.Stamina` _bpc_stats)) (not (`self.isDodging`)))
      (set `self.isDodging` true)
      (`|ExecutionSequence`
        (:`then_0`
          (if (`CharacterMovementComponent.bUseControllerDesiredRotation` (`Character.CharacterMovement` _player_bp))
            (bind _returnvalue (`/Game/ThirdPerson/Blueprints/BP_ThirdPersonCharacter.Get Movement Direction` _player_bp))
            (switch `int` (`KismetMathLibrary.Round` (/ _returnvalue 90.0))
              (:`-2`
                (set `self.Movement Direction` "NewEnumerator3" :!label _label_3))
              (:`-1`
                (set `self.Movement Direction` "NewEnumerator1"))
              (:`0`
                (set `self.Movement Direction` "NewEnumerator0" :!label _label_4))
              (:`1`
                (set `self.Movement Direction` "NewEnumerator2"))
              (:`2`
                (goto _label_3)))
            (else
              (goto _label_4))))
        (:`then_1`
          (`|PlayMontage` (`Character.Mesh` _player_bp) (select `/Game/Blueprints/E_MovementDirection` (`self.Movement Direction`) :`NewEnumerator0` "/Game/Characters/Souls/Combat/Dodge/Dodge_F_Montage.Dodge_F_Montage" :`NewEnumerator1` "/Game/Characters/Souls/Combat/Dodge/Dodge_L_Montage.Dodge_L_Montage" :`NewEnumerator3` "/Game/Characters/Souls/Combat/Dodge/Dodge_B_Montage.Dodge_B_Montage" :`NewEnumerator2` "/Game/Characters/Souls/Combat/Dodge/Dodge_R_Montage.Dodge_R_Montage" :!type "AnimMontage Object Reference")
            (:`then`
              (set `/Game/Blueprints/BPC_Stats.regainStamina` false _bpc_stats)
              (if (not (`/Game/ThirdPerson/Blueprints/BP_ThirdPersonCharacter.god mode` _player_bp))
                (`/Game/Blueprints/BPC_Stats.increase value` _bpc_stats "NewEnumerator1" (* _dodgestaminacost -1.0))))
            (:`OnCompleted`
              (set `self.isDodging` false :!label _label_5)
              (set `/Game/Blueprints/BPC_Stats.regainStamina` true _bpc_stats))
            (:`OnInterrupted`
              (goto _label_5))))))))