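; BPC_Stats is a stats component that tracks its owner's health and reports death.
; IncreaseValue switches on a stat type, adds the value to Health and clamps it between zero and MaxHealth.
; At zero health it fires Death, which sends DeathMessage to the owning actor.
; Each change also updates a health progress bar passed in through SetHealthProgressBar, if one is valid.
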(event `Death`
  (message `/Game/Blueprints/BPI_Damage.Death` (`self.GetOwner`)))

(event `Set Health Progress Bar`
  (params (`Health progress barNewParam` :type "ProgressBar Object Reference"))
  (set `self.Health Progress Bar New Param` `Health progress barNewParam`))

(fn `increase value`
  (params (Stat :type "/Game/Blueprints/E_Stats Enum" :default "NewEnumerator0") (Value :type "Float (double-precision)"))
  (bind _health (`self.health`))
  (bind _maxhealth (`self.maxHealth`))
  (switch `/Game/Blueprints/E_Stats` Stat
    (:`NewEnumerator0`
      (set `self.health` (`KismetMathLibrary.FClamp` (+ Value _health) 0.0 _maxhealth))
      (`|ExecutionSequence`
        (:`then_0`
          (if (<= _health 0.0)
            (`self.Death`)))
        (:`then_1`
          (bind _health_progress_bar_new_param (`self.Health Progress Bar New Param`)
            (:`then`
              (`ProgressBar.SetPercent` _health_progress_bar_new_param (/ _health _maxhealth)))
            (:`else`)))))))